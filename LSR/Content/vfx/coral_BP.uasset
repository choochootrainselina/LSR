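; Coral placement Blueprint that lines a spline with instances of a chosen coral mesh and material.
; The construction script derives spacing from the mesh's X bounds plus an offset, then fills the spline's length with instanced static meshes.
; A helper returns each instance's local location at that distance along the spline; rotation and scale stay at defaults, so instances do not follow the curve's direction.
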(fn `getTransformByIndex`
  (params (A :type "Float (double-precision)"))
  (returns (ReturnValue :type "Vector Structure"))
  (return (`SplineComponent.GetLocationAtDistanceAlongSpline` (`self.Spline`) (* (`KismetMathLibrary.Conv_IntToDouble` (`KismetMathLibrary.FTrunc` A)) (`self.spacing`)) "Local")))

(fn `UserConstructionScript`
  (bind _instancedstaticmesh (`self.InstancedStaticMesh`))
  (bind (_min _max) (break `Box` (`StaticMesh.GetBoundingBox` (`self.Coral Mesh`))))
  (`StaticMeshComponent.SetStaticMesh` (`self.InstancedStaticMesh`) (`self.Coral Mesh`))
  (bind _output_get (set `self.spacing` (+ (.x (- _max _min)) (`self.offset`))))
  (bind _output_get_2 (set `self.last index` (`KismetMathLibrary.FFloor` (/ (`SplineComponent.GetSplineLength` (`self.Spline`)) _output_get))))
  (for _index (range (+ _output_get_2 1))
    (bind _returnvalue (`self.getTransformByIndex` (`KismetMathLibrary.Conv_IntToDouble` _index)))
    (`PrimitiveComponent.SetMaterial` _instancedstaticmesh 0 (`self.Material`))
    (`InstancedStaticMeshComponent.AddInstance` _instancedstaticmesh (`KismetMathLibrary.MakeTransform` _returnvalue) false)))